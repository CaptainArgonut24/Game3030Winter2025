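; Enemy AI character that chases the player and damages them at close range.
; It halts its movement every tick until PawnSensing sees a pawn, which sets a seen flag and starts an AI move toward the player.
; On reaching the player, it subtracts Health directly on BP_ThirdPersonCharacter and plays a rifle-shoot montage.
; A CanAttack flag, reset on each sighting and after a montage-length delay, gates the attack.
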(event OnSeePawn(PawnSensing)
  (params (Pawn :type Pawn%20Object%20Reference))
  (Variables|Default|SetIsSEEPLAY true)
  (CallFunction|FollowPalyer))

(event Custom|Follow%20Palyer
  (Variables|Default|Setcan%20attack true)
  (if (Variables|Default|GetIsSEEPLAY)
    (AI|AIMoveTo self "0, 0, 0" (Game|GetPlayerCharacter 0) 7e+01 false
      (:then
        (if (Variables|Default|Getcan%20attack)
          (Variables|Default|Setcan%20attack false)
          (bind _asbp_third_person_character (Utilities|Casting|CastToBP_ThirdPersonCharacter (Game|GetPlayerCharacter 0)))
          (Variables|/Game/ThirdPerson/Blueprints/BP_ThirdPersonCharacter.BP_ThirdPersonCharacter_C|SetHealth _asbp_third_person_character (- (Variables|/Game/ThirdPerson/Blueprints/BP_ThirdPersonCharacter.BP_ThirdPersonCharacter_C|GetHealth _asbp_third_person_character) 0.2))
          (bind _returnvalue (Animation|PlayAnimMontage "/Game/FirstPersonArms/Animations/FP_Rifle_Shoot_Montage.FP_Rifle_Shoot_Montage" 1.0 "None"))
          (Utilities|FlowControl|Delay _returnvalue)
          (Variables|Default|Setcan%20attack true)
          (else
            (Variables|Default|SetIsSEEPLAY false)))))))

(event EventBeginPlay)

(event Collision|EventActorBeginOverlap
  (params (OtherActor :type Actor%20Object%20Reference)))

(event EventTick
  (params (DeltaSeconds :type Float%20%28single-precision%29))
  (if (not (Variables|Default|GetIsSEEPLAY))
    (Components|Movement|StopMovementImmediately (Variables|Character|GetCharacterMovement))))

(fn ConstructionScript)